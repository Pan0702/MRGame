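; Play button actor that loads a level when its OnCutFinished event fires.
; On BeginPlay it passes its LevelName to the WBP_LevelName user widget in its Widget component and prints debug success or failure messages.
; OnCutFinished starts a one-second camera fade and opens the referenced Play level immediately afterward, with no delay for the fade to finish.
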(event `self.ReceiveBeginPlay`
  (bind _aswbp_level_name (cast `/Game/MyData/Widget/WBP_LevelName` (`WidgetComponent.GetUserWidgetObject` (`self.Widget`)))
    (:`then`
      (set `/Game/MyData/Widget/WBP_LevelName.LevelText` (`self.LevelName`) _aswbp_level_name)
      (`KismetSystemLibrary.PrintString` "Success")
      (`KismetSystemLibrary.PrintString` (`KismetStringLibrary.Conv_NameToString` (`self.LevelName`))))
    (:`CastFailed`
      (`KismetSystemLibrary.PrintString` "Faild"))))

(event `self.OnCutFinished`
  (`PlayerCameraManager.StartCameraFade` :`self` (`GameplayStatics.GetPlayerCameraManager` 0) :`Duration` 1.0)
  (`GameplayStatics.OpenLevelBySoftObjectPtr` "/Game/Level/Play.Play"))

(fn `UserConstructionScript`)